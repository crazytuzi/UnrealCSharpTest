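; Unit test actor that checks Get, Set and Out functions for raw dynamic values called from Blueprint.
; On BeginPlay, a Sequence runs one group per type, from primitives, strings, enum and struct to object, class and soft references and containers, reporting each check to TestCoreSubsystem.
; Helpers TestSetEqual and TestMapEqual compare containers by length and content.
; Some struct and soft class checks read the member variable instead of the function result.
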(event `self.ReceiveBeginPlay`
  (`|ExecutionSequence`
    (:`then_0`
      (set `self.TestCoreSubsystem` (subsystem `TestCoreSubsystem`)))
    (:`then_1`
      (bind _none (`self.GetBoolValueFunction`))
      (`TestCoreSubsystem.TestEqual` (subsystem `TestCoreSubsystem`) "BlueprintRawDynamicGetBoolFunction" (== _none true))
      (`self.SetBoolValueFunction` false)
      (bind _none_2 (`self.GetBoolValueFunction`))
      (`TestCoreSubsystem.TestEqual` (subsystem `TestCoreSubsystem`) "BlueprintRawDynamicSetBoolFunction" (== _none_2 false))
      (`self.OutBoolValueFunction` (`self.OutBoolValue`))
      (`TestCoreSubsystem.TestEqual` (subsystem `TestCoreSubsystem`) "BlueprintRawDynamicOutBoolFunction" (== (`self.OutBoolValue`) false)))
    (:`then_2`
      (bind _none_3 (`self.GetInt32ValueFunction`))
      (`TestCoreSubsystem.TestEqual` (subsystem `TestCoreSubsystem`) "BlueprintRawDynamicGetInt32Function" (== _none_3 12))
      (`self.SetInt32ValueFunction` 21)
      (bind _none_4 (`self.GetInt32ValueFunction`))
      (`TestCoreSubsystem.TestEqual` (subsystem `TestCoreSubsystem`) "BlueprintRawDynamicSetInt32Function" (== _none_4 21))
      (`self.OutInt32ValueFunction` (`self.OutInt32Value`))
      (`TestCoreSubsystem.TestEqual` (subsystem `TestCoreSubsystem`) "BlueprintRawDynamicOutInt32Function" (== (`self.OutInt32Value`) 21)))
    (:`then_3`
      (bind _none_5 (`self.GetInt64ValueFunction`))
      (`TestCoreSubsystem.TestEqual` (subsystem `TestCoreSubsystem`) "BlueprintRawDynamicGetInt64Function" (== _none_5 12))
      (`self.SetInt64ValueFunction` 21)
      (bind _none_6 (`self.GetInt64ValueFunction`))
      (`TestCoreSubsystem.TestEqual` (subsystem `TestCoreSubsystem`) "BlueprintRawDynamicSetInt64Function" (== _none_6 21))
      (`self.OutInt64ValueFunction` (`self.OutInt64Value`))
      (`TestCoreSubsystem.TestEqual` (subsystem `TestCoreSubsystem`) "BlueprintRawDynamicOutInt64Function" (== (`self.OutInt64Value`) 21)))
    (:`then_4`
      (bind _none_7 (`self.GetUInt8ValueFunction`))
      (`TestCoreSubsystem.TestEqual` (subsystem `TestCoreSubsystem`) "BlueprintRawDynamicGetUInt8Function" (== _none_7 12))
      (`self.SetUInt8ValueFunction` 21)
      (bind _none_8 (`self.GetUInt8ValueFunction`))
      (`TestCoreSubsystem.TestEqual` (subsystem `TestCoreSubsystem`) "BlueprintRawDynamicSetUInt8Function" (== _none_8 21))
      (`self.OutUInt8ValueFunction` (`self.OutUInt8Value`))
      (`TestCoreSubsystem.TestEqual` (subsystem `TestCoreSubsystem`) "BlueprintRawDynamicOutUInt8Function" (== (`self.OutUInt8Value`) 21)))
    (:`then_5`
      (bind _none_9 (`self.GetDoubleValueFunction`))
      (`TestCoreSubsystem.TestEqual` (subsystem `TestCoreSubsystem`) "BlueprintRawDynamicGetDoubleFunction" (== _none_9 12.3))
      (`self.SetDoubleValueFunction` 3.21)
      (bind _none_10 (`self.GetDoubleValueFunction`))
      (`TestCoreSubsystem.TestEqual` (subsystem `TestCoreSubsystem`) "BlueprintRawDynamicSetDoubleFunction" (== _none_10 3.21))
      (`self.OutDoubleValueFunction` (`self.OutDoubleValue`))
      (`TestCoreSubsystem.TestEqual` (subsystem `TestCoreSubsystem`) "BlueprintRawDynamicOutDoubleFunction" (== (`self.OutDoubleValue`) 3.21)))
    (:`then_6`
      (bind _none_11 (`self.GetNameValueFunction`))
      (`TestCoreSubsystem.TestEqual` (subsystem `TestCoreSubsystem`) "BlueprintRawDynamicGetNameFunction" (== _none_11 "Name12"))
      (`self.SetNameValueFunction` "21emaN")
      (bind _none_12 (`self.GetNameValueFunction`))
      (`TestCoreSubsystem.TestEqual` (subsystem `TestCoreSubsystem`) "BlueprintRawDynamicSetNameFunction" (== _none_12 "21emaN"))
      (`self.OutNameValueFunction` (`self.OutNameValue`))
      (`TestCoreSubsystem.TestEqual` (subsystem `TestCoreSubsystem`) "BlueprintRawDynamicOutNameFunction" (== (`self.OutNameValue`) "21emaN")))
    (:`then_7`
      (bind _none_13 (`self.GetTextValueFunction`))
      (`TestCoreSubsystem.TestEqual` (subsystem `TestCoreSubsystem`) "BlueprintRawDynamicGetTextFunction" (`KismetTextLibrary.EqualEqual_TextText` _none_13 "Text12"))
      (`self.SetTextValueFunction` "21txeT")
      (bind _none_14 (`self.GetTextValueFunction`))
      (`TestCoreSubsystem.TestEqual` (subsystem `TestCoreSubsystem`) "BlueprintRawDynamicSetTextFunction" (`KismetTextLibrary.EqualEqual_TextText` _none_14 "21txeT"))
      (`self.OutTextValueFunction` (`self.OutTextValue`))
      (`TestCoreSubsystem.TestEqual` (subsystem `TestCoreSubsystem`) "BlueprintRawDynamicOutTextFunction" (`KismetTextLibrary.EqualEqual_TextText` (`self.OutTextValue`) "21txeT")))
    (:`then_8`
      (bind _none_15 (`self.GetStringValueFunction`))
      (`TestCoreSubsystem.TestEqual` (subsystem `TestCoreSubsystem`) "BlueprintRawDynamicGetStringFunction" (`KismetStringLibrary.EqualEqual_StrStr` _none_15 "String12"))
      (`self.SetStringValueFunction` "21gnirtS")
      (bind _none_16 (`self.GetStringValueFunction`))
      (`TestCoreSubsystem.TestEqual` (subsystem `TestCoreSubsystem`) "BlueprintRawDynamicSetStringFunction" (`KismetStringLibrary.EqualEqual_StrStr` _none_16 "21gnirtS"))
      (`self.OutStringValueFunction` (`self.OutStringValue`))
      (`TestCoreSubsystem.TestEqual` (subsystem `TestCoreSubsystem`) "BlueprintRawDynamicOutStringFunction" (`KismetStringLibrary.EqualEqual_StrStr` (`self.OutStringValue`) "21gnirtS")))
    (:`then_9`
      (bind _none_17 (`self.GetEnumValueFunction`))
      (`TestCoreSubsystem.TestEqual` (subsystem `TestCoreSubsystem`) "BlueprintRawDynamicGetEnumFunction" (`|EnumEquality` _none_17 "TestDynamicOne"))
      (`self.SetEnumValueFunction` "TestDynamicTwo")
      (bind _none_18 (`self.GetEnumValueFunction`))
      (`TestCoreSubsystem.TestEqual` (subsystem `TestCoreSubsystem`) "BlueprintRawDynamicSetEnumFunction" (`|EnumEquality` _none_18 "TestDynamicTwo"))
      (`self.OutEnumValueFunction` (`self.OutEnumValue`))
      (`TestCoreSubsystem.TestEqual` (subsystem `TestCoreSubsystem`) "BlueprintRawDynamicOutEnumFunction" (`|EnumEquality` (`self.OutEnumValue`) "TestDynamicTwo")))
    (:`then_10`
      (bind _none_19 (`self.GetStructValueFunction`))
      (`TestCoreSubsystem.TestEqual` (subsystem `TestCoreSubsystem`) "BlueprintRawDynamicGetStructFunction" (== (`.Value` (break `TestDynamicStruct` _none_19)) 1))
      (`self.SetStructValueFunction` (make `TestDynamicStruct` 2))
      (`self.GetStructValueFunction`)
      (`TestCoreSubsystem.TestEqual` (subsystem `TestCoreSubsystem`) "BlueprintRawDynamicSetStructFunction" (== (`.Value` (break `TestDynamicStruct` (`self.StructValue`))) 2))
      (set `self.OutStructValue` (make `TestDynamicStruct` 1))
      (`self.OutStructValueFunction` (`self.OutStructValue`))
      (`TestCoreSubsystem.TestEqual` (subsystem `TestCoreSubsystem`) "BlueprintRawDynamicOutStructFunction" (== (`.Value` (break `TestDynamicStruct` (`self.StructValue`))) 2)))
    (:`then_11`
      (bind _none_20 (`self.GetObjectValueFunction`))
      (`TestCoreSubsystem.TestEqual` (subsystem `TestCoreSubsystem`) "BlueprintRawDynamicGetObjectFunction" (== _none_20 self))
      (`self.SetObjectValueFunction` (subsystem `TestCoreSubsystem`))
      (bind _none_21 (`self.GetObjectValueFunction`))
      (`TestCoreSubsystem.TestEqual` (subsystem `TestCoreSubsystem`) "BlueprintRawDynamicSetObjectFunction" (== _none_21 (subsystem `TestCoreSubsystem`)))
      (set `self.OutObjectValue` self)
      (`self.OutObjectValueFunction` (`self.OutObjectValue`))
      (`TestCoreSubsystem.TestEqual` (subsystem `TestCoreSubsystem`) "BlueprintRawDynamicOutObjectFunction" (== (`self.OutObjectValue`) (subsystem `TestCoreSubsystem`))))
    (:`then_12`
      (bind _none_22 (`self.GetSubclassOfValueFunction`))
      (`TestCoreSubsystem.TestEqual` (subsystem `TestCoreSubsystem`) "BlueprintRawDynamicGetSubclassOfFunction" (== _none_22 (`GameplayStatics.GetObjectClass` self)))
      (`self.SetSubclassOfValueFunction` (`GameplayStatics.GetObjectClass` (subsystem `TestCoreSubsystem`)))
      (bind _none_23 (`self.GetSubclassOfValueFunction`))
      (`TestCoreSubsystem.TestEqual` (subsystem `TestCoreSubsystem`) "BlueprintRawDynamicSetSubclassOfFunction" (== _none_23 (`GameplayStatics.GetObjectClass` (subsystem `TestCoreSubsystem`))))
      (set `self.OutSubclassOfValue` (`GameplayStatics.GetObjectClass` self))
      (`self.OutSubclassOfValueFunction` (`self.OutSubclassOfValue`))
      (`TestCoreSubsystem.TestEqual` (subsystem `TestCoreSubsystem`) "BlueprintRawDynamicOutSubclassOfFunction" (== (`self.OutSubclassOfValue`) (`GameplayStatics.GetObjectClass` (subsystem `TestCoreSubsystem`)))))
    (:`then_13`
      (bind _none_24 (`self.GetSoftObjectPtrValueFunction`))
      (`TestCoreSubsystem.TestEqual` (subsystem `TestCoreSubsystem`) "BlueprintRawDynamicGetSoftObjectPtrFunction" (== _none_24 (`|ConvertAsset` self)))
      (`self.SetSoftObjectPtrValueFunction` (`|ConvertAsset` (subsystem `TestCoreSubsystem`)))
      (bind _none_25 (`self.GetSoftObjectPtrValueFunction`))
      (`TestCoreSubsystem.TestEqual` (subsystem `TestCoreSubsystem`) "BlueprintRawDynamicSetSoftObjectPtrFunction" (== _none_25 (`|ConvertAsset` (subsystem `TestCoreSubsystem`))))
      (set `self.OutSoftObjectPtrValue` (`|ConvertAsset` self))
      (`self.OutSoftObjectPtrValueFunction` (`self.OutSoftObjectPtrValue`))
      (`TestCoreSubsystem.TestEqual` (subsystem `TestCoreSubsystem`) "BlueprintRawDynamicOutSoftObjectPtrFunction" (== (`self.OutSoftObjectPtrValue`) (`|ConvertAsset` (subsystem `TestCoreSubsystem`)))))
    (:`then_14`
      (`self.GetSoftClassPtrValueFunction`)
      (`TestCoreSubsystem.TestEqual` (subsystem `TestCoreSubsystem`) "BlueprintRawDynamicGetSoftClassPtrFunction" (== (`self.SoftClassPtrValue`) (`|ConvertAsset` (`GameplayStatics.GetObjectClass` self))))
      (`self.SetSoftClassPtrValueFunction` (`|ConvertAsset` (`GameplayStatics.GetObjectClass` (subsystem `TestCoreSubsystem`))))
      (bind _none_26 (`self.GetSoftClassPtrValueFunction`))
      (`TestCoreSubsystem.TestEqual` (subsystem `TestCoreSubsystem`) "BlueprintRawDynamicSetSoftClassPtrFunction" (== _none_26 (`|ConvertAsset` (`GameplayStatics.GetObjectClass` (subsystem `TestCoreSubsystem`)))))
      (set `self.OutSoftClassPtrValue` (`|ConvertAsset` (`GameplayStatics.GetObjectClass` self)))
      (`self.OutSoftClassPtrValueFunction` (`self.OutSoftClassPtrValue`))
      (`TestCoreSubsystem.TestEqual` (subsystem `TestCoreSubsystem`) "BlueprintRawDynamicOutSoftClassPtrFunction" (== (`self.OutSoftClassPtrValue`) (`|ConvertAsset` (`GameplayStatics.GetObjectClass` (subsystem `TestCoreSubsystem`))))))
    (:`then_15`
      (bind _none_27 (`self.GetArrayValueFunction`))
      (`TestCoreSubsystem.TestEqual` (subsystem `TestCoreSubsystem`) "BlueprintRawDynamicGetArrayFunction" (`KismetArrayLibrary.Array_Identical` _none_27 (`|MakeArray` 1 2)))
      (`self.SetArrayValueFunction` (`|MakeArray` 3 4))
      (bind _none_28 (`self.GetArrayValueFunction`))
      (`TestCoreSubsystem.TestEqual` (subsystem `TestCoreSubsystem`) "BlueprintRawDynamicSetArrayFunction" (`KismetArrayLibrary.Array_Identical` _none_28 (`|MakeArray` 3 4)))
      (`self.OutArrayValueFunction` (`self.OutArrayValue`))
      (`TestCoreSubsystem.TestEqual` (subsystem `TestCoreSubsystem`) "BlueprintRawDynamicOutArrayFunction" (`KismetArrayLibrary.Array_Identical` (`self.OutArrayValue`) (`|MakeArray` 3 4))))
    (:`then_16`
      (bind _none_29 (`self.GetSetValueFunction`))
      (`TestCoreSubsystem.TestEqual` (subsystem `TestCoreSubsystem`) "BlueprintRawDynamicGetSetFunction" (`self.TestSetEqual` _none_29 (`|MakeSet` 1 2)))
      (`self.SetSetValueFunction` (`|MakeSet` 3 4))
      (bind _none_30 (`self.GetSetValueFunction`))
      (`TestCoreSubsystem.TestEqual` (subsystem `TestCoreSubsystem`) "BlueprintRawDynamicSetSetFunction" (`self.TestSetEqual` _none_30 (`|MakeSet` 3 4)))
      (`self.OutSetValueFunction` (`self.OutSetValue`))
      (`TestCoreSubsystem.TestEqual` (subsystem `TestCoreSubsystem`) "BlueprintRawDynamicOutSetFunction" (`self.TestSetEqual` (`self.OutSetValue`) (`|MakeSet` 3 4))))
    (:`then_17`
      (bind _none_31 (`self.GetMapValueFunction`))
      (`TestCoreSubsystem.TestEqual` (subsystem `TestCoreSubsystem`) "BlueprintRawDynamicGetMapFunction" (`self.TestMapEqual` _none_31 (`|MakeMap` 1 1 2 2)))
      (`self.SetMapValueFunction` (`|MakeMap` 3 3 4 4))
      (bind _none_32 (`self.GetMapValueFunction`))
      (`TestCoreSubsystem.TestEqual` (subsystem `TestCoreSubsystem`) "BlueprintRawDynamicSetMapFunction" (`self.TestMapEqual` _none_32 (`|MakeMap` 3 3 4 4)))
      (`self.OutMapValueFunction` (`self.OutMapValue`))
      (`TestCoreSubsystem.TestEqual` (subsystem `TestCoreSubsystem`) "BlueprintRawDynamicOutMapFunction" (`self.TestMapEqual` (`self.OutMapValue`) (`|MakeMap` 3 3 4 4))))))

(fn `TestMapEqual`
  (params (InActual :type "Map of Integer to Integer") (InExpected :type "Map of Integer to Integer"))
  (returns (ReturnValue :type Boolean))
  (if (== (`BlueprintMapLibrary.Map_Length` InActual) (`BlueprintMapLibrary.Map_Length` InExpected))
    (bind _keys (`BlueprintMapLibrary.Map_Keys` InActual))
    (for _array_element _keys
      (bind (_value _returnvalue) (`BlueprintMapLibrary.Map_Find` InExpected _array_element))
      (if _returnvalue
        (if (not (== (`BlueprintMapLibrary.Map_Find` InActual _array_element) _value))
          (return false))
        (else
          (return false))))
    (return true)
    (else
      (return false))))

(fn `TestSetEqual`
  (params (InActual :type "Set of Integer") (InExpected :type "Set of Integer"))
  (returns (ReturnValue :type Boolean))
  (if (== (`BlueprintSetLibrary.Set_Length` InActual) (`BlueprintSetLibrary.Set_Length` InExpected))
    (bind _result (`BlueprintSetLibrary.Set_ToArray` InActual))
    (for _array_element _result
      (if (not (`BlueprintSetLibrary.Set_Contains` InExpected _array_element))
        (return false)))
    (return true)
    (else
      (return false))))

(fn `UserConstructionScript`)