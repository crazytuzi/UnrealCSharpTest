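; Unit test actor that checks Blueprint get and set access to dynamic properties of many types, from primitives, text, enum and struct to object, class and soft references and containers.
; On BeginPlay, a sequence asserts each variable's expected initial value, assigns a new one and asserts again, reporting named results to TestCoreSubsystem.
; Helper functions TestSetEqual and TestMapEqual compare sets and maps by length and per-element lookup.
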(event `self.ReceiveBeginPlay`
  (`|ExecutionSequence`
    (:`then_0`
      (`TestCoreSubsystem.TestEqual` (subsystem `TestCoreSubsystem`) "BlueprintBlueprintDynamicGetBoolProperty" (== (`self.BoolValue`) true))
      (set `self.BoolValue` false)
      (`TestCoreSubsystem.TestEqual` (subsystem `TestCoreSubsystem`) "BlueprintBlueprintDynamicSetBoolProperty" (== (`self.BoolValue`) false)))
    (:`then_1`
      (`TestCoreSubsystem.TestEqual` (subsystem `TestCoreSubsystem`) "BlueprintBlueprintDynamicGetInt32Property" (== (`self.Int32Value`) 12))
      (set `self.Int32Value` 21)
      (`TestCoreSubsystem.TestEqual` (subsystem `TestCoreSubsystem`) "BlueprintBlueprintDynamicSetInt32Property" (== (`self.Int32Value`) 21)))
    (:`then_2`
      (`TestCoreSubsystem.TestEqual` (subsystem `TestCoreSubsystem`) "BlueprintBlueprintDynamicGetInt64Property" (== (`self.Int64Value`) 12))
      (set `self.Int64Value` 21)
      (`TestCoreSubsystem.TestEqual` (subsystem `TestCoreSubsystem`) "BlueprintBlueprintDynamicSetInt64Property" (== (`self.Int64Value`) 21)))
    (:`then_3`
      (`TestCoreSubsystem.TestEqual` (subsystem `TestCoreSubsystem`) "BlueprintBlueprintDynamicGetUInt8Property" (== (`self.UInt8Value`) 12))
      (set `self.UInt8Value` 21)
      (`TestCoreSubsystem.TestEqual` (subsystem `TestCoreSubsystem`) "BlueprintBlueprintDynamicSetUInt8Property" (== (`self.UInt8Value`) 21)))
    (:`then_4`
      (`TestCoreSubsystem.TestEqual` (subsystem `TestCoreSubsystem`) "BlueprintBlueprintDynamicGetDoubleProperty" (== (`self.DoubleValue`) 12.3))
      (set `self.DoubleValue` 3.21)
      (`TestCoreSubsystem.TestEqual` (subsystem `TestCoreSubsystem`) "BlueprintBlueprintDynamicSetDoubleProperty" (== (`self.DoubleValue`) 3.21)))
    (:`then_5`
      (`TestCoreSubsystem.TestEqual` (subsystem `TestCoreSubsystem`) "BlueprintBlueprintDynamicGetNameProperty" (== (`self.NameValue`) "Name12"))
      (set `self.NameValue` "21emaN")
      (`TestCoreSubsystem.TestEqual` (subsystem `TestCoreSubsystem`) "BlueprintBlueprintDynamicSetNameProperty" (== (`self.NameValue`) "21emaN")))
    (:`then_6`
      (`TestCoreSubsystem.TestEqual` (subsystem `TestCoreSubsystem`) "BlueprintBlueprintDynamicGetTextProperty" (`KismetTextLibrary.EqualEqual_TextText` (`self.TextValue`) "Text12"))
      (set `self.TextValue` "21txeT")
      (`TestCoreSubsystem.TestEqual` (subsystem `TestCoreSubsystem`) "BlueprintBlueprintDynamicSetTextProperty" (`KismetTextLibrary.EqualEqual_TextText` (`self.TextValue`) "21txeT")))
    (:`then_7`
      (`TestCoreSubsystem.TestEqual` (subsystem `TestCoreSubsystem`) "BlueprintBlueprintDynamicGetStringProperty" (`KismetStringLibrary.EqualEqual_StrStr` (`self.StringValue`) "String12"))
      (set `self.StringValue` "21gnirtS")
      (`TestCoreSubsystem.TestEqual` (subsystem `TestCoreSubsystem`) "BlueprintBlueprintDynamicSetStringProperty" (`KismetStringLibrary.EqualEqual_StrStr` (`self.StringValue`) "21gnirtS")))
    (:`then_8`
      (`TestCoreSubsystem.TestEqual` (subsystem `TestCoreSubsystem`) "BlueprintBlueprintDynamicGetEnumProperty" (`|EnumEquality` (`self.EnumValue`) "TestDynamicOne"))
      (set `self.EnumValue` "TestDynamicTwo")
      (`TestCoreSubsystem.TestEqual` (subsystem `TestCoreSubsystem`) "BlueprintBlueprintDynamicSetEnumProperty" (`|EnumEquality` (`self.EnumValue`) "TestDynamicTwo")))
    (:`then_9`
      (`TestCoreSubsystem.TestEqual` (subsystem `TestCoreSubsystem`) "BlueprintBlueprintDynamicGetStructProperty" (== (`.Value` (break `TestDynamicStruct` (`self.StructValue`))) 1))
      (set `self.StructValue` (make `TestDynamicStruct` 0 0 2))
      (`TestCoreSubsystem.TestEqual` (subsystem `TestCoreSubsystem`) "BlueprintBlueprintDynamicSetStructProperty" (== (`.Value` (break `TestDynamicStruct` (`self.StructValue`))) 2)))
    (:`then_10`
      (`TestCoreSubsystem.TestEqual` (subsystem `TestCoreSubsystem`) "BlueprintBlueprintDynamicGetObjectProperty" (== (`self.ObjectValue`) self))
      (set `self.ObjectValue` (subsystem `TestCoreSubsystem`))
      (`TestCoreSubsystem.TestEqual` (subsystem `TestCoreSubsystem`) "BlueprintBlueprintDynamicSetObjectProperty" (== (`self.ObjectValue`) (subsystem `TestCoreSubsystem`))))
    (:`then_11`
      (`TestCoreSubsystem.TestEqual` (subsystem `TestCoreSubsystem`) "BlueprintBlueprintDynamicGetSubclassOfProperty" (== (`self.SubclassOfValue`) (`GameplayStatics.GetObjectClass` self)))
      (set `self.SubclassOfValue` (`GameplayStatics.GetObjectClass` (subsystem `TestCoreSubsystem`)))
      (`TestCoreSubsystem.TestEqual` (subsystem `TestCoreSubsystem`) "BlueprintBlueprintDynamicSetSubclassOfProperty" (== (`self.SubclassOfValue`) (`GameplayStatics.GetObjectClass` (subsystem `TestCoreSubsystem`)))))
    (:`then_12`
      (`TestCoreSubsystem.TestEqual` (subsystem `TestCoreSubsystem`) "BlueprintBlueprintDynamicGetSoftObjectPtrProperty" (== (`self.SoftObjectPtrValue`) (`|ConvertAsset` self)))
      (set `self.SoftObjectPtrValue` (`|ConvertAsset` (subsystem `TestCoreSubsystem`)))
      (`TestCoreSubsystem.TestEqual` (subsystem `TestCoreSubsystem`) "BlueprintBlueprintDynamicSetSoftObjectPtrProperty" (== (`self.SoftObjectPtrValue`) (`|ConvertAsset` (subsystem `TestCoreSubsystem`)))))
    (:`then_13`
      (`TestCoreSubsystem.TestEqual` (subsystem `TestCoreSubsystem`) "BlueprintBlueprintDynamicGetSoftClassPtrProperty" (== (`self.SoftClassPtrValue`) (`|ConvertAsset` (`GameplayStatics.GetObjectClass` self))))
      (set `self.SoftClassPtrValue` (`|ConvertAsset` (`GameplayStatics.GetObjectClass` (subsystem `TestCoreSubsystem`))))
      (`TestCoreSubsystem.TestEqual` (subsystem `TestCoreSubsystem`) "BlueprintBlueprintDynamicSetSoftClassPtrProperty" (== (`self.SoftClassPtrValue`) (`|ConvertAsset` (`GameplayStatics.GetObjectClass` (subsystem `TestCoreSubsystem`))))))
    (:`then_14`
      (`TestCoreSubsystem.TestEqual` (subsystem `TestCoreSubsystem`) "BlueprintBlueprintDynamicGetArrayProperty" (`KismetArrayLibrary.Array_Identical` (`self.ArrayValue`) (`|MakeArray` 1 2)))
      (set `self.ArrayValue` (`|MakeArray` 3 4))
      (`TestCoreSubsystem.TestEqual` (subsystem `TestCoreSubsystem`) "BlueprintBlueprintDynamicSetArrayProperty" (`KismetArrayLibrary.Array_Identical` (`self.ArrayValue`) (`|MakeArray` 3 4))))
    (:`then_15`
      (`TestCoreSubsystem.TestEqual` (subsystem `TestCoreSubsystem`) "BlueprintBlueprintDynamicGetSetProperty" (`self.TestSetEqual` (`self.SetValue`) (`|MakeSet` 1 2)))
      (set `self.SetValue` (`|MakeSet` 3 4))
      (`TestCoreSubsystem.TestEqual` (subsystem `TestCoreSubsystem`) "BlueprintBlueprintDynamicSetSetProperty" (`self.TestSetEqual` (`self.SetValue`) (`|MakeSet` 3 4))))
    (:`then_16`
      (`TestCoreSubsystem.TestEqual` (subsystem `TestCoreSubsystem`) "BlueprintBlueprintDynamicGetMapProperty" (`self.TestMapEqual` (`self.MapValue`) (`|MakeMap` 1 1 2 2)))
      (set `self.MapValue` (`|MakeMap` 3 3 4 4))
      (`TestCoreSubsystem.TestEqual` (subsystem `TestCoreSubsystem`) "BlueprintBlueprintDynamicSetMapProperty" (`self.TestMapEqual` (`self.MapValue`) (`|MakeMap` 3 3 4 4))))))

(fn `TestMapEqual`
  (params (InActual :type "Map of Integer to Integer") (InExpected :type "Map of Integer to Integer"))
  (returns (ReturnValue :type Boolean))
  (if (== (`BlueprintMapLibrary.Map_Length` InActual) (`BlueprintMapLibrary.Map_Length` InExpected))
    (bind _keys (`BlueprintMapLibrary.Map_Keys` InActual))
    (for _array_element _keys
      (bind (_value _returnvalue) (`BlueprintMapLibrary.Map_Find` InExpected _array_element))
      (if _returnvalue
        (if (not (== (`BlueprintMapLibrary.Map_Find` InActual _array_element) _value))
          (return false))
        (else
          (return false))))
    (return true)
    (else
      (return false))))

(fn `TestSetEqual`
  (params (InActual :type "Set of Integer") (InExpected :type "Set of Integer"))
  (returns (ReturnValue :type Boolean))
  (if (== (`BlueprintSetLibrary.Set_Length` InActual) (`BlueprintSetLibrary.Set_Length` InExpected))
    (bind _result (`BlueprintSetLibrary.Set_ToArray` InActual))
    (for _array_element _result
      (if (not (`BlueprintSetLibrary.Set_Contains` InExpected _array_element))
        (return false)))
    (return true)
    (else
      (return false))))

(fn `UserConstructionScript`)