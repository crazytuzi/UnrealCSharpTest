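; Unit test actor that verifies Blueprint get and set access to raw dynamic properties of many types, from primitives to object references, structs and containers.
; On BeginPlay, a sequence checks each property's expected initial value, assigns a new one and re-checks it, reporting to TestCoreSubsystem.
; The interface property is only reassigned to itself, so its set check expects the same object.
; TestSetEqual and TestMapEqual helpers compare containers by length and contents, ignoring order.
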(event `self.ReceiveBeginPlay`
  (`|ExecutionSequence`
    (:`then_0`
      (`TestCoreSubsystem.TestEqual` (subsystem `TestCoreSubsystem`) "BlueprintRawDynamicGetBoolProperty" (== (`self.BoolValue`) true))
      (set `self.BoolValue` false)
      (`TestCoreSubsystem.TestEqual` (subsystem `TestCoreSubsystem`) "BlueprintRawDynamicSetBoolProperty" (== (`self.BoolValue`) false)))
    (:`then_1`
      (`TestCoreSubsystem.TestEqual` (subsystem `TestCoreSubsystem`) "BlueprintRawDynamicGetInt32Property" (== (`self.Int32Value`) 12))
      (set `self.Int32Value` 21)
      (`TestCoreSubsystem.TestEqual` (subsystem `TestCoreSubsystem`) "BlueprintRawDynamicSetInt32Property" (== (`self.Int32Value`) 21)))
    (:`then_2`
      (`TestCoreSubsystem.TestEqual` (subsystem `TestCoreSubsystem`) "BlueprintRawDynamicGetInt64Property" (== (`self.Int64Value`) 12))
      (set `self.Int64Value` 21)
      (`TestCoreSubsystem.TestEqual` (subsystem `TestCoreSubsystem`) "BlueprintRawDynamicSetInt64Property" (== (`self.Int64Value`) 21)))
    (:`then_3`
      (`TestCoreSubsystem.TestEqual` (subsystem `TestCoreSubsystem`) "BlueprintRawDynamicGetUInt8Property" (== (`self.UInt8Value`) 12))
      (set `self.UInt8Value` 21)
      (`TestCoreSubsystem.TestEqual` (subsystem `TestCoreSubsystem`) "BlueprintRawDynamicSetUInt8Property" (== (`self.UInt8Value`) 21)))
    (:`then_4`
      (`TestCoreSubsystem.TestEqual` (subsystem `TestCoreSubsystem`) "BlueprintRawDynamicGetDoubleProperty" (== (`self.DoubleValue`) 12.3))
      (set `self.DoubleValue` 3.21)
      (`TestCoreSubsystem.TestEqual` (subsystem `TestCoreSubsystem`) "BlueprintRawDynamicSetDoubleProperty" (== (`self.DoubleValue`) 3.21)))
    (:`then_5`
      (`TestCoreSubsystem.TestEqual` (subsystem `TestCoreSubsystem`) "BlueprintRawDynamicGetNameProperty" (== (`self.NameValue`) "Name12"))
      (set `self.NameValue` "21emaN")
      (`TestCoreSubsystem.TestEqual` (subsystem `TestCoreSubsystem`) "BlueprintRawDynamicSetNameProperty" (== (`self.NameValue`) "21emaN")))
    (:`then_6`
      (`TestCoreSubsystem.TestEqual` (subsystem `TestCoreSubsystem`) "BlueprintRawDynamicGetTextProperty" (`KismetTextLibrary.EqualEqual_TextText` (`self.TextValue`) "Text12"))
      (set `self.TextValue` "21txeT")
      (`TestCoreSubsystem.TestEqual` (subsystem `TestCoreSubsystem`) "BlueprintRawDynamicSetTextProperty" (`KismetTextLibrary.EqualEqual_TextText` (`self.TextValue`) "21txeT")))
    (:`then_7`
      (`TestCoreSubsystem.TestEqual` (subsystem `TestCoreSubsystem`) "BlueprintRawDynamicGetStringProperty" (`KismetStringLibrary.EqualEqual_StrStr` (`self.StringValue`) "String12"))
      (set `self.StringValue` "21gnirtS")
      (`TestCoreSubsystem.TestEqual` (subsystem `TestCoreSubsystem`) "BlueprintRawDynamicSetStringProperty" (`KismetStringLibrary.EqualEqual_StrStr` (`self.StringValue`) "21gnirtS")))
    (:`then_8`
      (`TestCoreSubsystem.TestEqual` (subsystem `TestCoreSubsystem`) "BlueprintRawDynamicGetEnumProperty" (`|EnumEquality` (`self.EnumValue`) "TestDynamicOne"))
      (set `self.EnumValue` "TestDynamicTwo")
      (`TestCoreSubsystem.TestEqual` (subsystem `TestCoreSubsystem`) "BlueprintRawDynamicSetEnumProperty" (`|EnumEquality` (`self.EnumValue`) "TestDynamicTwo")))
    (:`then_9`
      (`TestCoreSubsystem.TestEqual` (subsystem `TestCoreSubsystem`) "BlueprintRawDynamicGetStructProperty" (== (`.Value` (break `TestDynamicStruct` (`self.StructValue`))) 1))
      (set `self.StructValue` (make `TestDynamicStruct` 2))
      (`TestCoreSubsystem.TestEqual` (subsystem `TestCoreSubsystem`) "BlueprintRawDynamicSetStructProperty" (== (`.Value` (break `TestDynamicStruct` (`self.StructValue`))) 2)))
    (:`then_10`
      (`TestCoreSubsystem.TestEqual` (subsystem `TestCoreSubsystem`) "BlueprintRawDynamicGetObjectProperty" (== (`self.ObjectValue`) self))
      (set `self.ObjectValue` (subsystem `TestCoreSubsystem`))
      (`TestCoreSubsystem.TestEqual` (subsystem `TestCoreSubsystem`) "BlueprintRawDynamicSetObjectProperty" (== (`self.ObjectValue`) (subsystem `TestCoreSubsystem`))))
    (:`then_11`
      (`TestCoreSubsystem.TestEqual` (subsystem `TestCoreSubsystem`) "BlueprintRawDynamicGetInterfaceProperty" (== (`KismetSystemLibrary.Conv_InterfaceToObject` (`self.InterfaceValue`)) self))
      (set `self.InterfaceValue` (`self.InterfaceValue`))
      (`TestCoreSubsystem.TestEqual` (subsystem `TestCoreSubsystem`) "BlueprintRawDynamicSetInterfaceProperty" (== (`KismetSystemLibrary.Conv_InterfaceToObject` (`self.InterfaceValue`)) self)))
    (:`then_12`
      (`TestCoreSubsystem.TestEqual` (subsystem `TestCoreSubsystem`) "BlueprintRawDynamicGetSubclassOfProperty" (== (`self.SubclassOfValue`) (`GameplayStatics.GetObjectClass` self)))
      (set `self.SubclassOfValue` (`GameplayStatics.GetObjectClass` (subsystem `TestCoreSubsystem`)))
      (`TestCoreSubsystem.TestEqual` (subsystem `TestCoreSubsystem`) "BlueprintRawDynamicSetSubclassOfProperty" (== (`self.SubclassOfValue`) (`GameplayStatics.GetObjectClass` (subsystem `TestCoreSubsystem`)))))
    (:`then_13`
      (`TestCoreSubsystem.TestEqual` (subsystem `TestCoreSubsystem`) "BlueprintRawDynamicGetSoftObjectPtrProperty" (== (`self.SoftObjectPtrValue`) (`|ConvertAsset` self)))
      (set `self.SoftObjectPtrValue` (`|ConvertAsset` (subsystem `TestCoreSubsystem`)))
      (`TestCoreSubsystem.TestEqual` (subsystem `TestCoreSubsystem`) "BlueprintRawDynamicSetSoftObjectPtrProperty" (== (`self.SoftObjectPtrValue`) (`|ConvertAsset` (subsystem `TestCoreSubsystem`)))))
    (:`then_14`
      (`TestCoreSubsystem.TestEqual` (subsystem `TestCoreSubsystem`) "BlueprintRawDynamicGetSoftClassPtrProperty" (== (`self.SoftClassPtrValue`) (`|ConvertAsset` (`GameplayStatics.GetObjectClass` self))))
      (set `self.SoftClassPtrValue` (`|ConvertAsset` (`GameplayStatics.GetObjectClass` (subsystem `TestCoreSubsystem`))))
      (`TestCoreSubsystem.TestEqual` (subsystem `TestCoreSubsystem`) "BlueprintRawDynamicSetSoftClassPtrProperty" (== (`self.SoftClassPtrValue`) (`|ConvertAsset` (`GameplayStatics.GetObjectClass` (subsystem `TestCoreSubsystem`))))))
    (:`then_15`
      (`TestCoreSubsystem.TestEqual` (subsystem `TestCoreSubsystem`) "BlueprintRawDynamicGetArrayProperty" (`KismetArrayLibrary.Array_Identical` (`self.ArrayValue`) (`|MakeArray` 1 2)))
      (set `self.ArrayValue` (`|MakeArray` 3 4))
      (`TestCoreSubsystem.TestEqual` (subsystem `TestCoreSubsystem`) "BlueprintRawDynamicSetArrayProperty" (`KismetArrayLibrary.Array_Identical` (`self.ArrayValue`) (`|MakeArray` 3 4))))
    (:`then_16`
      (`TestCoreSubsystem.TestEqual` (subsystem `TestCoreSubsystem`) "BlueprintRawDynamicGetSetProperty" (`self.TestSetEqual` (`self.SetValue`) (`|MakeSet` 1 2)))
      (set `self.SetValue` (`|MakeSet` 3 4))
      (`TestCoreSubsystem.TestEqual` (subsystem `TestCoreSubsystem`) "BlueprintRawDynamicSetSetProperty" (`self.TestSetEqual` (`self.SetValue`) (`|MakeSet` 3 4))))
    (:`then_17`
      (`TestCoreSubsystem.TestEqual` (subsystem `TestCoreSubsystem`) "BlueprintRawDynamicGetMapProperty" (`self.TestMapEqual` (`self.MapValue`) (`|MakeMap` 1 1 2 2)))
      (set `self.MapValue` (`|MakeMap` 3 3 4 4))
      (`TestCoreSubsystem.TestEqual` (subsystem `TestCoreSubsystem`) "BlueprintRawDynamicSetMapProperty" (`self.TestMapEqual` (`self.MapValue`) (`|MakeMap` 3 3 4 4))))))

(fn `TestMapEqual`
  (params (InActual :type "Map of Integer to Integer") (InExpected :type "Map of Integer to Integer"))
  (returns (ReturnValue :type Boolean))
  (if (== (`BlueprintMapLibrary.Map_Length` InActual) (`BlueprintMapLibrary.Map_Length` InExpected))
    (bind _keys (`BlueprintMapLibrary.Map_Keys` InActual))
    (for _array_element _keys
      (bind (_value _returnvalue) (`BlueprintMapLibrary.Map_Find` InExpected _array_element))
      (if _returnvalue
        (if (not (== (`BlueprintMapLibrary.Map_Find` InActual _array_element) _value))
          (return false))
        (else
          (return false))))
    (return true)
    (else
      (return false))))

(fn `TestSetEqual`
  (params (InActual :type "Set of Integer") (InExpected :type "Set of Integer"))
  (returns (ReturnValue :type Boolean))
  (if (== (`BlueprintSetLibrary.Set_Length` InActual) (`BlueprintSetLibrary.Set_Length` InExpected))
    (bind _result (`BlueprintSetLibrary.Set_ToArray` InActual))
    (for _array_element _result
      (if (not (`BlueprintSetLibrary.Set_Contains` InExpected _array_element))
        (return false)))
    (return true)
    (else
      (return false))))

(fn `UserConstructionScript`)