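; Unit-test actor fixture for reflection, exposing Blueprint functions over member variables of many property types, apparently for calls from C#.
; Each type, from primitives, strings and enums to structs, objects, classes, interfaces and containers, has a Set, a Get and an Out function.
; Out functions write the stored value through a by-ref parameter.
; BeginPlay seeds ObjectValue with self and InterfaceValue with self cast to BP_TestInterface.
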(event `self.ReceiveBeginPlay`
  (set `self.ObjectValue` self)
  (bind _asbp_test_interface (cast `/Game/UnitTest/Core/BP_TestInterface` self))
  (set `self.InterfaceValue` _asbp_test_interface))

(fn `GetArrayValueFunction`
  (returns (ReturnValue :type "Array of Integer"))
  (return (`self.ArrayValue`)))

(fn `GetBoolValueFunction`
  (returns (ReturnValue :type Boolean))
  (return (`self.BoolValue`)))

(fn `GetClassValueFunction`
  (returns (ReturnValue :type "Object Class Reference"))
  (return (`self.ClassValue`)))

(fn `GetDoubleValueFunction`
  (returns (ReturnValue :type "Float (double-precision)"))
  (return (`self.DoubleValue`)))

(fn `GetEnumValueFunction`
  (returns (ReturnValue :type "/Game/UnitTest/Core/BP_TestEnum Enum"))
  (return (`self.EnumValue`)))

(fn `GetInt32ValueFunction`
  (returns (ReturnValue :type Integer))
  (return (`self.Int32Value`)))

(fn `GetInt64ValueFunction`
  (returns (ReturnValue :type Integer64))
  (return (`self.Int64Value`)))

(fn `GetInterfaceValueFunction`
  (returns (ReturnValue :type "/Game/UnitTest/Core/BP_TestInterface Interface"))
  (return (`self.InterfaceValue`)))

(fn `GetMapValueFunction`
  (returns (ReturnValue :type "Map of Integer to Integer"))
  (return (`self.MapValue`)))

(fn `GetNameValueFunction`
  (returns (ReturnValue :type Name))
  (return (`self.NameValue`)))

(fn `GetObjectValueFunction`
  (returns (ReturnValue :type "Object Object Reference"))
  (return (`self.ObjectValue`)))

(fn `GetSetValueFunction`
  (returns (ReturnValue :type "Set of Integer"))
  (return (`self.SetValue`)))

(fn `GetStringValueFunction`
  (returns (ReturnValue :type String))
  (return (`self.StringValue`)))

(fn `GetStructValueFunction`
  (returns (ReturnValue :type "/Game/UnitTest/Core/BP_TestStruct Structure"))
  (return (`self.StructValue`)))

(fn `GetTextValueFunction`
  (returns (ReturnValue :type Text))
  (return (`self.TextValue`)))

(fn `GetUInt8ValueFunction`
  (returns (ReturnValue :type Byte))
  (return (`self.UInt8Value`)))

(fn `OutArrayValueFunction`
  (params (OutArrayValue :type "Array of Integer"))
  (`|VariableSetRef` OutArrayValue (`self.ArrayValue`)))

(fn `OutBoolValueFunction`
  (params (OutBoolValue :type "Boolean (by ref)"))
  (`|VariableSetRef` OutBoolValue (`self.BoolValue`)))

(fn `OutClassValueFunction`
  (params (OutClassValue :type "Object Class Reference (by ref)"))
  (`|VariableSetRef` OutClassValue (`self.ClassValue`)))

(fn `OutDoubleValueFunction`
  (params (OutDoubleValue :type "Float (double-precision) (by ref)"))
  (`|VariableSetRef` OutDoubleValue (`self.DoubleValue`)))

(fn `OutEnumValueFunction`
  (params (OutEnumValue :type "/Game/UnitTest/Core/BP_TestEnum Enum (by ref)"))
  (`|VariableSetRef` OutEnumValue (`self.EnumValue`)))

(fn `OutInt32ValueFunction`
  (params (OutInt32Value :type "Integer (by ref)"))
  (`|VariableSetRef` OutInt32Value (`self.Int32Value`)))

(fn `OutInt64ValueFunction`
  (params (OutInt64Value :type "Integer64 (by ref)"))
  (`|VariableSetRef` OutInt64Value (`self.Int64Value`)))

(fn `OutInterfaceValueFunction`
  (params (OutInterfaceValue :type "/Game/UnitTest/Core/BP_TestInterface Interface (by ref)"))
  (`|VariableSetRef` OutInterfaceValue (`self.InterfaceValue`)))

(fn `OutMapValueFunction`
  (params (OutMapValue :type "Map of Integer to Integer (by ref)"))
  (`|VariableSetRef` OutMapValue (`self.MapValue`)))

(fn `OutNameValueFunction`
  (params (OutNameValue :type "Name (by ref)"))
  (`|VariableSetRef` OutNameValue (`self.NameValue`)))

(fn `OutObjectValueFunction`
  (params (OutObjectValue :type "Object Object Reference (by ref)"))
  (`|VariableSetRef` OutObjectValue (`self.ObjectValue`)))

(fn `OutSetValueFunction`
  (params (OutSetValue :type "Set of Integer (by ref)"))
  (`|VariableSetRef` OutSetValue (`self.SetValue`)))

(fn `OutStringValueFunction`
  (params (OutStringValue :type "String (by ref)"))
  (`|VariableSetRef` OutStringValue (`self.StringValue`)))

(fn `OutStructValueFunction`
  (params (OutStructValue :type "/Game/UnitTest/Core/BP_TestStruct Structure (by ref)"))
  (`|VariableSetRef` OutStructValue (`self.StructValue`)))

(fn `OutTextValueFunction`
  (params (OutTextValue :type "Text (by ref)"))
  (`|VariableSetRef` OutTextValue (`self.TextValue`)))

(fn `OutUInt8ValueFunction`
  (params (OutUInt8Value :type "Byte (by ref)"))
  (`|VariableSetRef` OutUInt8Value (`self.UInt8Value`)))

(fn `SetArrayValueFunction`
  (params (InArrayValue :type "Array of Integer"))
  (set `self.ArrayValue` InArrayValue))

(fn `SetBoolValueFunction`
  (params (InBoolValue :type Boolean))
  (set `self.BoolValue` InBoolValue))

(fn `SetClassValueFunction`
  (params (InClassValue :type "Object Class Reference"))
  (set `self.ClassValue` InClassValue))

(fn `SetDoubleValueFunction`
  (params (InDoubleValue :type "Float (double-precision)"))
  (set `self.DoubleValue` InDoubleValue))

(fn `SetEnumValueFunction`
  (params (InEnumValue :type "/Game/UnitTest/Core/BP_TestEnum Enum" :default "NewEnumerator0"))
  (set `self.EnumValue` InEnumValue))

(fn `SetInt32ValueFunction`
  (params (InInt32Value :type Integer))
  (set `self.Int32Value` InInt32Value))

(fn `SetInt64ValueFunction`
  (params (InInt64Value :type Integer64))
  (set `self.Int64Value` InInt64Value))

(fn `SetInterfaceValueFunction`
  (params (InInterfaceValue :type "/Game/UnitTest/Core/BP_TestInterface Interface"))
  (set `self.InterfaceValue` InInterfaceValue))

(fn `SetMapValueFunction`
  (params (InMapValue :type "Map of Integer to Integer"))
  (set `self.MapValue` InMapValue))

(fn `SetNameValueFunction`
  (params (InNameValue :type Name))
  (set `self.NameValue` InNameValue))

(fn `SetObjectValueFunction`
  (params (InObjectValue :type "Object Object Reference"))
  (set `self.ObjectValue` InObjectValue))

(fn `SetSetValueFunction`
  (params (InSetValue :type "Set of Integer"))
  (set `self.SetValue` InSetValue))

(fn `SetStringValueFunction`
  (params (InStringValue :type String))
  (set `self.StringValue` InStringValue))

(fn `SetStructValueFunction`
  (params (InStructValue :type "/Game/UnitTest/Core/BP_TestStruct Structure"))
  (set `self.StructValue` InStructValue))

(fn `SetTextValueFunction`
  (params (InTextValue :type Text))
  (set `self.TextValue` InTextValue))

(fn `SetUInt8ValueFunction`
  (params (InUInt8Value :type Byte))
  (set `self.UInt8Value` InUInt8Value))

(fn `UserConstructionScript`)